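; Generated dynamic mesh actor that procedurally builds a snow layer over a chosen set of actors.
; On rebuild it merges their root meshes in world space, then casts seeded random downward rays through a BVH.
; Each hit adds a scaled sphere box, and the result is moved into actor-local space.
; Optional remeshing uses morphology and smoothing to blend the snow, then rebuilds UVs, tangents and normals.
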(event `self.OnRebuildGeneratedMesh`
  (params (TargetMesh :type "DynamicMesh Object Reference"))
  (bind _stream (`self.Stream`))
  (set `self.Target Mesh` TargetMesh)
  (`|ExecutionSequence`
    (:`then_0`
      ; get mesh and add it to \n array
      (bind _returnvalue (`self.AllocateComputeMesh`))
      (set `self.raycast_mesh` _returnvalue)
      (for _array_element (`self.meshes_to_add_snow_to`)
        (bind _returnvalue_2 (`self.AllocateComputeMesh`))
        (bind (_localtoworld _returnvalue_3) (`GeometryScriptLibrary_SceneUtilityFunctions.CopyMeshFromComponent` (`Actor.RootComponent` _array_element) _returnvalue_2 (struct) true null)
          (:`Failure`
            _)
          (:`Success`
            _))
        (`self.ReleaseComputeMesh` null)
        (`GeometryScriptLibrary_MeshBasicEditFunctions.AppendMesh` (`self.raycast_mesh`) _returnvalue_3 (struct) false (struct :`CombineMode` "EnableAllMatching") null)))
    (:`then_1`
      ; add random raycast and create snow
      (bind (_outputbvh _returnvalue_4) (`GeometryScriptLibrary_MeshSpatial.BuildBVHForMesh` (`self.raycast_mesh`) null))
      (set `self.Output BVH` _outputbvh)
      (for _ (range (+ (`self.number of snow`) 1))
        (bind _returnvalue_5 (`GeometryScriptLibrary_MeshQueryFunctions.GetMeshBoundingBox` _returnvalue_4))
        (bind _hitresult (`GeometryScriptLibrary_MeshSpatial.FindNearestRayIntersectionWithMesh` (`self.raycast_mesh`) (`self.Output BVH`) (`KismetMathLibrary.MakeVector` (`KismetMathLibrary.RandomFloatInRangeFromStream` _stream (.x (break `Box` _returnvalue_5)) (.x (`.Max` (break `Box` _returnvalue_5)))) (`KismetMathLibrary.RandomFloatInRangeFromStream` _stream (.y (break `Box` _returnvalue_5)) (.y (`.Max` (break `Box` _returnvalue_5)))) (+ (- (.z (break `Box` _returnvalue_5)) (.z (`.Max` (break `Box` _returnvalue_5)))) (`self.height of snowfall`))) (0.0 0.0 -1.0) (struct) null)
          (:`Found`
            (`GeometryScriptLibrary_MeshPrimitiveFunctions.AppendSphereBox` (`self.Target Mesh`) (struct) (`KismetMathLibrary.MakeTransform` (`.HitPosition` (break `GeometryScriptRayHitResult` _hitresult)) (struct) (`self.snow shape`)) 50.0 6 6 6 "Center" null)))))
    (:`then_2`
      ; anchor pivot point to array
      (`GeometryScriptLibrary_MeshTransformFunctions.TransformMesh` (`self.Target Mesh`) (`KismetMathLibrary.InvertTransform` (`self.GetTransform`)) true null))
    (:`then_3`
      ; smoth and shape snow
      (if (`self.remesh`)
        (bind _returnvalue_6 (`GeometryScriptLibrary_MeshVoxelFunctions.ApplyMeshMorphology` (`self.Target Mesh`) (make `GeometryScriptMorphologyOptions` (make `GeometryScript3DGridParameters` "GridResolution") false (make `GeometryScript3DGridParameters` "GridResolution") (struct :`Min` (0.0 0.0 0.0) :`Max` (0.0 0.0 0.0)) "Dilate" (`self.snow_depth`)) null))
        (bind _returnvalue_7 (`GeometryScriptLibrary_MeshDeformFunctions.ApplyIterativeSmoothingToMesh` _returnvalue_6 (struct) (make `GeometryScriptIterativeMeshSmoothingOptions` (`self.smoothness`)) null))
        (bind (_returnvalue_min _returnvalue_max) (break `Box` (`GeometryScriptLibrary_MeshQueryFunctions.GetMeshBoundingBox` _returnvalue_7)))
        (bind _returnvalue_8 (`GeometryScriptLibrary_MeshUVFunctions.SetMeshUVsFromBoxProjection` _returnvalue_7 0 (`KismetMathLibrary.MakeTransform` (0.0 0.0 0.0) (struct) (- _returnvalue_max _returnvalue_min)) (struct) 2 null))
        (bind _returnvalue_9 (`GeometryScriptLibrary_MeshNormalsFunctions.ComputeTangents` _returnvalue_8 (struct) null))
        (`GeometryScriptLibrary_MeshNormalsFunctions.ComputeSplitNormals` _returnvalue_9 (make `GeometryScriptSplitNormalsOptions` true 80.0) (struct) null)))
    (:`then_4`
      ; clear unused meshes from memory
      (`self.ReleaseAllComputeMeshes`))
    (:`then_5`
      ; import niagra snowfall
      (set `self.height of snowfall` (`self.height of snowfall`)))))

(fn `UserConstructionScript`)